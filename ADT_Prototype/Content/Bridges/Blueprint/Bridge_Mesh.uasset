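; Modular bridge actor that assembles itself along its Y axis from static mesh components in the Construction Script.
; It repeats entrance and center spans by a set count and adds road extensions at both ends.
; A shape switch picks between two styles of entrance and pillars, and a depth setting stacks cement columns downward.
; At runtime, a one-second delay loop from BeginPlay destroys the bridge once the player pawn is over 30000 units away.
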(event EventBeginPlay
  (if (> (Math|Vector|VectorLength (- (Transformation|GetActorLocation (Game|Player|GetPlayerPawn 0)) (Transformation|GetActorLocation))) 3e+04) :!label _label
    (Actor|DestroyActor)
    (else
      (Utilities|FlowControl|Delay 1.0)
      (goto _label))))

(fn ConstructionScript
  (bind _number_of_times_the_bridge_is_repeated (Variables|Default|GetNumber_of_times_the_bridge_is_repeated))
  (CallFunction|BridgeEntrance 0.0)
  (for _index (range 1 _number_of_times_the_bridge_is_repeated)
    (CallFunction|BridgeCenter (+ 2.4e+04 (* _index -2.64e+04)))
    (CallFunction|BridgeEntrance (* _index -2.64e+04)))
  (for _index_2 (range 1 (Variables|Default|GetExtension_of_the_bridge_from_the_first_side))
    (CallFunction|PartOftheRoad (* _index_2 2.4e+03)))
  (for _index_3 (range 1 (Variables|Default|GetExtension_of_the_bridge_from_the_second_side))
    (CallFunction|PartOftheRoad (+ (* _index_3 -2.4e+03) (* _number_of_times_the_bridge_is_repeated -2.64e+04)))))

(fn BridgeEntrance
  (params (Y%20Location :type Float%20%28double-precision%29))
  (CallFunction|PartOftheRoad Y%20Location)
  (AddComponent|AddStaticMeshComponent false (Math|Transform|MakeTransform (Math|Vector|MakeVector -1.1e+03 Y%20Location 0.0) "0,180.000000, 0" "1.000000,1.000000,1.000000"))
  (for _index (range 0 (Variables|Default|GetExtend_the_depth_of_the_cement_columns))
    (AddComponent|AddStaticMeshComponent false (Math|Transform|MakeTransform (Math|Vector|MakeVector -1.1e+03 Y%20Location (* _index -1e+03)) "0,180.000000, 0" "1.000000,1.000000,1.000000"))
    (switch Utilities|FlowControl|Switch|SwitchonEN_BridgeShape (Variables|Default|GetBridge_shape)
      (:NewEnumerator0
        (LocalVariables|SetFirst%20index 0)
        (LocalVariables|SetLast%20index 9))
      (:NewEnumerator1
        (LocalVariables|SetFirst%20index 10)
        (LocalVariables|SetLast%20index 14)))
    (for _index_2 (range (LocalVariables|GetFirst%20index) (LocalVariables|GetLast%20index))
      (bind _returnvalue (AddComponent|AddStaticMeshComponent false (Math|Transform|MakeTransform (Math|Vector|MakeVector -1.1e+03 Y%20Location 0.0) "0,180.000000, 0" "1.000000,1.000000,1.000000")))
      (Components|StaticMesh|SetStaticMesh _returnvalue (Utilities|Array|Get(acopy) (Variables|Default|GetStatic_mesh_bridge_entrance) _index_2)))))

(fn PartOftheRoad
  (params (Y%20Location :type Float%20%28double-precision%29))
  (bind _returnvalue (- Y%20Location 1.2e+03))
  (AddComponent|AddStaticMeshComponent false (Math|Transform|MakeTransform (Math|Vector|MakeVector 1.1e+03 Y%20Location 0.0) "0, 0, 0" "1.000000,1.000000,1.000000"))
  (AddComponent|AddStaticMeshComponent false (Math|Transform|MakeTransform (Math|Vector|MakeVector 1.05e+03 _returnvalue 8e+01) "0,180.000000, 0" "1.000000,1.000000,1.000000"))
  (AddComponent|AddStaticMeshComponent false (Math|Transform|MakeTransform (Math|Vector|MakeVector -1.05e+03 _returnvalue 8e+01) "0, 0, 0" "1.000000,1.000000,1.000000"))
  (AddComponent|AddStaticMeshComponent false (Math|Transform|MakeTransform (Math|Vector|MakeVector 0.0 _returnvalue 8e+01) "0, 0, 0" "1.000000,1.000000,1.000000"))
  (for _index (range -5 0)
    (AddComponent|AddStaticMeshComponent false (Math|Transform|MakeTransform (Math|Vector|MakeVector 1027.0 (+ (* _index 4e+02) -2e+02 Y%20Location) 8e+01) "0, 0, 0" "1.000000,1.000000,1.000000"))
    (AddComponent|AddStaticMeshComponent false (Math|Transform|MakeTransform (Math|Vector|MakeVector -1027.0 (+ (* _index 4e+02) -2e+02 Y%20Location) 8e+01) "0,180.000000, 0" "1.000000,1.000000,1.000000"))))

(fn BridgeCenter
  (params (Y%20Location :type Float%20%28double-precision%29))
  (for _index (range 0 9)
    (CallFunction|PartOftheRoad (+ (* _index -2.4e+03) Y%20Location)))
  (CallFunction|LowerPillars Y%20Location)
  (CallFunction|UpperPillars Y%20Location))

(fn LowerPillars
  (params (Y%20Location :type Float%20%28double-precision%29))
  (for _array_element (Variables|Default|GetStatic_mesh_bridge_center_lower_pillars)
    (bind _returnvalue (AddComponent|AddStaticMeshComponent false (Math|Transform|MakeTransform (Math|Vector|MakeVector 0.0 (- Y%20Location 1.2e+04) 0.0) "0, 0, 0" "1.000000,1.000000,1.000000")))
    (Components|StaticMesh|SetStaticMesh _returnvalue _array_element))
  (switch Utilities|FlowControl|Switch|SwitchonEN_BridgeShape (Variables|Default|GetBridge_shape)
    (:NewEnumerator0
      (for _index (range 0 9)
        (AddComponent|AddStaticMeshComponent false (Math|Transform|MakeTransform (Math|Vector|MakeVector 0.0 (+ (* _index -2.4e+03) -1.2e+03 Y%20Location) 0.0) "0, 0, 0" "1.000000,1.000000,1.000000"))
        (AddComponent|AddStaticMeshComponent false (Math|Transform|MakeTransform (Math|Vector|MakeVector 0.0 (+ (* _index -2.4e+03) -1.2e+03 Y%20Location) 0.0) "0,180.000000, 0" "1.000000,1.000000,1.000000"))))))

(fn UpperPillars
  (params (Y%20Location :type Float%20%28double-precision%29))
  (bind _returnvalue (+ -1.2e+04 Y%20Location))
  (bind _returnvalue_2 (Math|Vector|MakeVector 0.0 _returnvalue 0.0))
  (switch Utilities|FlowControl|Switch|SwitchonEN_BridgeShape (Variables|Default|GetBridge_shape)
    (:NewEnumerator0
      (for _array_element (Variables|Default|GetStatic_mesh_bridge_center_upper_pillars)
        (bind _returnvalue_3 (AddComponent|AddStaticMeshComponent false (Math|Transform|MakeTransform _returnvalue_2 "0, 0, 0" "1.000000,1.000000,1.000000")))
        (Components|StaticMesh|SetStaticMesh _returnvalue_3 _array_element)
        (bind _returnvalue_4 (AddComponent|AddStaticMeshComponent false (Math|Transform|MakeTransform _returnvalue_2 "0,180.000000, 0" "1.000000,1.000000,1.000000")))
        (Components|StaticMesh|SetStaticMesh _returnvalue_4 _array_element)))
    (:NewEnumerator1
      (for _index (range 0 9)
        (AddComponent|AddStaticMeshComponent false (Math|Transform|MakeTransform (Math|Vector|MakeVector 1.16e+03 (+ (* _index -2.4e+03) Y%20Location) -8e+01) "0, 0, 0" "1.000000,1.000000,1.000000"))
        (AddComponent|AddStaticMeshComponent false (Math|Transform|MakeTransform (Math|Vector|MakeVector 1.16e+03 (+ (* _index -2.4e+03) Y%20Location) -8e+01) "0, 0, 0" "1.000000,1.000000,1.000000"))
        (AddComponent|AddStaticMeshComponent false (Math|Transform|MakeTransform (Math|Vector|MakeVector -1.16e+03 (+ (* _index -2.4e+03) Y%20Location) -8e+01) "0, 0, 0" "1.000000,1.000000,1.000000"))
        (AddComponent|AddStaticMeshComponent false (Math|Transform|MakeTransform (Math|Vector|MakeVector -1.16e+03 (+ (* _index -2.4e+03) Y%20Location) -8e+01) "0, 0, 0" "1.000000,1.000000,1.000000"))))))