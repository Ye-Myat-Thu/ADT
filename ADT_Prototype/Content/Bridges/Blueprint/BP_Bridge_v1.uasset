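; Procedural bridge actor that assembles its static mesh components entirely in the construction script, with no runtime logic.
; Fixed-spacing loops lay the central road and barriers, while BridgeShape picks one of three index ranges from a pillar mesh array.
; Mirrored end sections add road, pillars, lamppost-line meshes and stacked cement columns of adjustable depth.
; Two exposed counts repeat approach segments to extend either side of the bridge independently.
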(event EventBeginPlay)

(event Collision|EventActorBeginOverlap
  (params (OtherActor :type Actor%20Object%20Reference)))

(event EventTick
  (params (DeltaSeconds :type Float%20%28single-precision%29)))

(fn ConstructionScript
  (CallFunction|AddRoadinBridge)
  (CallFunction|AddBarrierinBridge)
  (CallFunction|AddPillarinBridge)
  (CallFunction|AddPillarandRoad)
  (CallFunction|TheBeginningandEndOftheBridge))

(fn AddRoadinBridge
  (for _index (range -4 5)
    (AddComponent|AddStaticMeshComponent false (Math|Transform|MakeTransform (Math|Vector|MakeVector 7e+02 (* _index 2.4e+03) 0.0) "0, 0, 0" "1.000000,1.000000,1.000000"))
    (AddComponent|AddStaticMeshComponent false (Math|Transform|MakeTransform (Math|Vector|MakeVector 7e+02 (* _index 2.4e+03) 0.0) "0, 0, 0" "1.000000,1.000000,1.000000"))
    (AddComponent|AddStaticMeshComponent false (Math|Transform|MakeTransform (Math|Vector|MakeVector 6.5e+02 (- (* _index 2.4e+03) 1.2e+03) 8e+01) "0,180.000000, 0" "1.000000,1.000000,1.000000"))
    (AddComponent|AddStaticMeshComponent false (Math|Transform|MakeTransform (Math|Vector|MakeVector -6.5e+02 (- (* _index 2.4e+03) 1.2e+03) 8e+01) "0,0.000000, 0" "1.000000,1.000000,1.000000"))))

(fn AddBarrierinBridge
  (for _index (range -29 30)
    (AddComponent|AddStaticMeshComponent false (Math|Transform|MakeTransform (Math|Vector|MakeVector 627.0 (+ (* _index 4e+02) -2e+02) 8e+01) "0, 0, 0" "1.000000,1.000000,1.000000"))
    (AddComponent|AddStaticMeshComponent false (Math|Transform|MakeTransform (Math|Vector|MakeVector -627.0 (+ (* _index 4e+02) -2e+02) 8e+01) "0,180.000000, 0" "1.000000,1.000000,1.000000"))))

(fn AddPillarinBridge
  (switch Utilities|FlowControl|Switch|SwitchonEN_BridgeShape (Variables|Default|GetBridge%20shape)
    (:NewEnumerator0
      (LocalVariables|SetFirst%20index 0)
      (LocalVariables|SetLast%20index 27))
    (:NewEnumerator1
      (LocalVariables|SetFirst%20index 28)
      (LocalVariables|SetLast%20index 48))
    (:NewEnumerator2
      (LocalVariables|SetFirst%20index 49)
      (LocalVariables|SetLast%20index 92)))
  (for _index (range (LocalVariables|GetFirst%20index) (LocalVariables|GetLast%20index))
    (bind _returnvalue (AddComponent|AddStaticMeshComponent false))
    (Components|StaticMesh|SetStaticMesh _returnvalue (Utilities|Array|Get(acopy) (Variables|Default|GetStatic_Mesh_Pillar_Bridge) _index))))

(fn AddPillarandRoad
  (for _index (range 0 1)
    (switch int _index
      (:0
        (LocalVariables|SetLamppost_Location -1.35e+04)
        (LocalVariables|SetTransformComponent (Math|Transform|MakeTransform "700.000000,-12000.000000,0.000000" "0, 0,0.000000" "1.000000,1.000000,1.000000")))
      (:1
        (LocalVariables|SetLamppost_Location 1.35e+04)
        (LocalVariables|SetTransformComponent (Math|Transform|MakeTransform "-700.000000,12000.000000,0.000000" "0.000000,180.000000,0.000000" "1.000000,1.000000,1.000000"))))
    (for _index_2 (range 0 3)
      (bind _returnvalue (AddComponent|AddStaticMeshComponent false (LocalVariables|GetTransformComponent)))
      (Components|StaticMesh|SetStaticMesh _returnvalue (Utilities|Array|Get(acopy) (Variables|Default|GetStatic_Mesh_Road_and_pillar) _index_2)))
    (AddComponent|AddStaticMeshComponent false (Math|Transform|MakeTransform (Math|Vector|MakeVector 0.0 (LocalVariables|GetLamppost_Location) 8e+01) "0, 0, 0" "1.000000,1.000000,1.000000"))
    (AddComponent|AddStaticMeshComponent false (Math|Transform|MakeTransform (Math|Vector|MakeVector -1.05e+03 (LocalVariables|GetLamppost_Location) 8e+01) "0, 0, 0" "1.000000,1.000000,1.000000"))
    (AddComponent|AddStaticMeshComponent false (Math|Transform|MakeTransform (Math|Vector|MakeVector 1.05e+03 (LocalVariables|GetLamppost_Location) 8e+01) "0,180.000000, 0" "1.000000,1.000000,1.000000"))
    (for _index_3 (range 1 (Variables|Default|GetExtend_the_depth_of_the_cement_columns))
      (AddComponent|AddStaticMeshComponent false (Math|Transform|MakeTransform (Math|Vector|MakeVector (.x (.location (LocalVariables|GetTransformComponent))) (.y (.location (LocalVariables|GetTransformComponent))) (+ (* _index_3 -1097.0) (.z (.location (LocalVariables|GetTransformComponent))))) (.rotation (LocalVariables|GetTransformComponent)) (.scale (LocalVariables|GetTransformComponent))))))
  (for _index_4 (range 0 2)
    (AddComponent|AddStaticMeshComponent false (Math|Transform|MakeTransform (Math|Vector|MakeVector -1027.0 (+ (* _index_4 4e+02) -1.42e+04) 8e+01) "0,180.000000, 0" "1.000000,1.000000,1.000000"))
    (AddComponent|AddStaticMeshComponent false (Math|Transform|MakeTransform (Math|Vector|MakeVector 1027.0 (+ (* _index_4 4e+02) -1.42e+04) 8e+01) "0,0.000000, 0" "1.000000,1.000000,1.000000"))
    (AddComponent|AddStaticMeshComponent false (Math|Transform|MakeTransform (Math|Vector|MakeVector -1027.0 (* (+ (* _index_4 4e+02) -1.42e+04) -1.0) 8e+01) "0,180.000000, 0" "1.000000,1.000000,1.000000"))
    (AddComponent|AddStaticMeshComponent false (Math|Transform|MakeTransform (Math|Vector|MakeVector 1027.0 (* (+ (* _index_4 4e+02) -1.42e+04) -1.0) 8e+01) "0,0.000000, 0" "1.000000,1.000000,1.000000"))))

(fn TheBeginningandEndOftheBridge
  (for _index (range 0 (Variables|Default|GetExtension_of_the_bridge_from_the_first_side))
    (AddComponent|AddStaticMeshComponent false (Math|Transform|MakeTransform (Math|Vector|MakeVector 1.1e+03 (+ 1.68e+04 (* _index 2.4e+03)) 0.0) "0, 0, 0" "1.000000,1.000000,1.000000"))
    (for _index_2 (range 0 5)
      (AddComponent|AddStaticMeshComponent false (Math|Transform|MakeTransform (Math|Vector|MakeVector -1027.0 (+ (* _index_2 -4e+02) 1.66e+04 (* _index 2.4e+03)) 8e+01) "0,180.000000, 0" "1.000000,1.000000,1.000000"))
      (AddComponent|AddStaticMeshComponent false (Math|Transform|MakeTransform (Math|Vector|MakeVector 1027.0 (+ (* _index_2 -4e+02) 1.66e+04 (* _index 2.4e+03)) 8e+01) "0,0.000000, 0" "1.000000,1.000000,1.000000"))
      (AddComponent|AddStaticMeshComponent false (Math|Transform|MakeTransform (Math|Vector|MakeVector 0.0 (+ (* _index 2.4e+03) 1.59e+04) 8e+01) "0, 0, 0" "1.000000,1.000000,1.000000"))
      (AddComponent|AddStaticMeshComponent false (Math|Transform|MakeTransform (Math|Vector|MakeVector -1.05e+03 (+ (* _index 2.4e+03) 1.59e+04) 8e+01) "0, 0, 0" "1.000000,1.000000,1.000000"))
      (AddComponent|AddStaticMeshComponent false (Math|Transform|MakeTransform (Math|Vector|MakeVector 1.05e+03 (+ (* _index 2.4e+03) 1.59e+04) 8e+01) "0,180.000000, 0" "1.000000,1.000000,1.000000"))))
  (for _index_3 (range 0 (Variables|Default|GetExtension_of_the_bridge_from_the_second_side))
    (AddComponent|AddStaticMeshComponent false (Math|Transform|MakeTransform (Math|Vector|MakeVector -1.1e+03 (+ -1.68e+04 (* _index_3 -2.4e+03)) 0.0) "0,180.000000, 0" "1.000000,1.000000,1.000000"))
    (for _index_4 (range 0 5)
      (AddComponent|AddStaticMeshComponent false (Math|Transform|MakeTransform (Math|Vector|MakeVector -1027.0 (+ (* _index_4 4e+02) -1.66e+04 (* _index_3 -2.4e+03)) 8e+01) "0,180.000000, 0" "1.000000,1.000000,1.000000"))
      (AddComponent|AddStaticMeshComponent false (Math|Transform|MakeTransform (Math|Vector|MakeVector 1027.0 (+ (* _index_4 4e+02) -1.66e+04 (* _index_3 -2.4e+03)) 8e+01) "0,0.000000, 0" "1.000000,1.000000,1.000000"))
      (AddComponent|AddStaticMeshComponent false (Math|Transform|MakeTransform (Math|Vector|MakeVector 0.0 (+ (* _index_3 -2.4e+03) -1.59e+04) 8e+01) "0, 0, 0" "1.000000,1.000000,1.000000"))
      (AddComponent|AddStaticMeshComponent false (Math|Transform|MakeTransform (Math|Vector|MakeVector -1.05e+03 (+ (* _index_3 -2.4e+03) -1.59e+04) 8e+01) "0, 0, 0" "1.000000,1.000000,1.000000"))
      (AddComponent|AddStaticMeshComponent false (Math|Transform|MakeTransform (Math|Vector|MakeVector 1.05e+03 (+ (* _index_3 -2.4e+03) -1.59e+04) 8e+01) "0,180.000000, 0" "1.000000,1.000000,1.000000")))))